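; Player character for a three-lane dodging game, switching between left, center and right lanes and jumping over or avoiding obstacles.
; Q and D update the current side stored in BP_GameState and pick that lane's X target, while Space drives jumping.
; Tick interpolates X toward the target and pins Y to a hardcoded value.
; Hitting a BP_Obstacle shows the EndScreen widget, guarded by DoOnce.
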(event `self.ReceiveBeginPlay`
  (set `self.GameStateRef` (cast `/Game/Content/Blueprints/game/BP_GameState` (`GameplayStatics.GetGameState`) :!pure true)))

(event `Key|D`
  (params (Key :type "Key Structure"))
  (bind _gamestateref (`self.GameStateRef`))
  (bind _rightlocation (`/Game/Content/Blueprints/game/BP_GameState.RightLocation` _gamestateref))
  (:`Pressed`
    (set `self.TargetXLocation` (select `/Game/Content/Enum/EWhichSide` (`/Game/Content/Blueprints/game/BP_GameState.CurrentSide` (`self.GameStateRef`)) :`NewEnumerator0` _rightlocation :`NewEnumerator1` (`/Game/Content/Blueprints/game/BP_GameState.CenterLocation` _gamestateref) :`NewEnumerator2` _rightlocation))
    (set `/Game/Content/Blueprints/game/BP_GameState.CurrentSide` (select `/Game/Content/Enum/EWhichSide` (`/Game/Content/Blueprints/game/BP_GameState.CurrentSide` (`self.GameStateRef`)) :`NewEnumerator0` "NewEnumerator2" :`NewEnumerator1` "NewEnumerator0" :`NewEnumerator2` "NewEnumerator2" :!type "/Game/Content/Enum/EWhichSide Enum") (`self.GameStateRef`))))

(event `Key|Q`
  (params (Key :type "Key Structure"))
  (bind _gamestateref (`self.GameStateRef`))
  (bind _leftlocation (`/Game/Content/Blueprints/game/BP_GameState.LeftLocation` _gamestateref))
  (:`Pressed`
    (set `self.TargetXLocation` (select `/Game/Content/Enum/EWhichSide` (`/Game/Content/Blueprints/game/BP_GameState.CurrentSide` (`self.GameStateRef`)) :`NewEnumerator0` _leftlocation :`NewEnumerator1` _leftlocation :`NewEnumerator2` (`/Game/Content/Blueprints/game/BP_GameState.CenterLocation` _gamestateref)))
    (set `/Game/Content/Blueprints/game/BP_GameState.CurrentSide` (select `/Game/Content/Enum/EWhichSide` (`/Game/Content/Blueprints/game/BP_GameState.CurrentSide` (`self.GameStateRef`)) :`NewEnumerator0` "NewEnumerator1" :`NewEnumerator1` "NewEnumerator1" :`NewEnumerator2` "NewEnumerator0" :!type "/Game/Content/Enum/EWhichSide Enum") (`self.GameStateRef`))))

(event `self.ReceiveTick`
  (params (DeltaSeconds :type "Float (single-precision)"))
  (bind _returnvalue_x (`KismetMathLibrary.BreakVector` (`self.K2_GetActorLocation`)))
  (bind (_returnvalue_x_2 _returnvalue_y _returnvalue_z) (`KismetMathLibrary.BreakVector` (`self.K2_GetActorLocation`)))
  (`self.K2_SetActorLocation` (`KismetMathLibrary.MakeVector` (`KismetMathLibrary.FInterpTo` _returnvalue_x (`self.TargetXLocation`) DeltaSeconds (`self.SideWaySpeed`)) -1453.880801 _returnvalue_z)))

(event `Key|SpaceBar`
  (params (Key :type "Key Structure"))
  (:`Pressed`
    (`self.Jump`)
    (set `self.IsJumping` true))
  (:`Released`
    (`self.StopJumping`)
    (set `self.IsJumping` false)))

(event `self.ReceiveHit`
  (params (MyComp :type "PrimitiveComponent Object Reference") (Other :type "Actor Object Reference") (OtherComp :type "PrimitiveComponent Object Reference") (bSelfMoved :type Boolean) (HitLocation :type "Vector Structure") (HitNormal :type "Vector Structure") (NormalImpulse :type "Vector Structure") (Hit :type "HitResult Structure (by ref)"))
  (cast `/Game/Content/Blueprints/game/Course/Obstacles/BP_Obstacle` Other)
  (`/Engine/EditorBlueprintResources/StandardMacros.DoOnce` false
    (:`Completed`
      (bind _returnvalue (`|CreateWidget` "/Game/Content/UI/EndScreen.EndScreen_C"))
      (`UserWidget.AddToViewport` _returnvalue 0))))

(fn `UserConstructionScript`)